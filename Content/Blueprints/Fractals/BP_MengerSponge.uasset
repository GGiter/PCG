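; Menger sponge fractal actor, built from cube instances in the construction script and spun in pitch on Tick.
; Each iteration after the first shrinks spacing and size by three, calls GenerateBoxes repeatedly, then removes entries from Points by index.
; GenerateBoxes adds the 20 outer cells of a 3x3x3 grid, centred on the origin rather than a parent box.
; SpawnBoxes adds the points to HISMActor as world-space instances.
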(event Collision|EventActorBeginOverlap
  (params (OtherActor :type Actor%20Object%20Reference)))

(event EventTick
  (params (DeltaSeconds :type Float%20%28single-precision%29))
  (Transformation|AddActorLocalRotation (Math|Rotator|MakeRotator 0.0 (* DeltaSeconds (Variables|Default|GetSpeed)) 0.0) false false))

(fn ConstructionScript
  (bind _points (Variables|Default|GetPoints))
  (for _index (range 1 (Variables|Default|GetNumOfIterations))
    (if (> _index 1)
      (Variables|Default|SetNumOfBoxes (Math|Float|Truncate (Math|Float|Power (Math|Conversions|ToFloat(Integer) (- _index 1)) 2e+01)))
      (Variables|Default|Setr (/ (Variables|Default|Getr) 3.0))
      (Variables|Default|SetSizeR (/ (Variables|Default|GetSizeR) 3.0))
      (for _index_2 (range 1 (Variables|Default|GetNumOfBoxes))
        (CallFunction|GenerateBoxes))
      (for _index_3 (range 0 (- (Variables|Default|GetToDelete) 1))
        (if (Utilities|Array|IsValidIndex _points _index_3)
          (Utilities|Array|RemoveIndex _points _index_3)))
      (Variables|Default|SetToDelete (* (Variables|Default|GetToDelete) 20))))
  (CallFunction|SpawnBoxes))

(fn GenerateBoxes
  (params (BoxIndex :type Integer))
  (bind _r (Variables|Default|Getr))
  (bind _sizer (Variables|Default|GetSizeR))
  (for _index (range -1 1)
    (for _index_2 (range -1 1)
      (for _index_3 (range -1 1)
        (if (> (+ (+ (Math|Integer|Absolute(Integer) _index) (Math|Integer|Absolute(Integer) _index_2)) (Math|Integer|Absolute(Integer) _index_3)) 1)
          (Utilities|Array|Add (Variables|Default|GetPoints) (Math|Transform|MakeTransform (Math|Vector|MakeVector (* _index _r) (* _index_2 _r) (* _index_3 _r)) "0, 0, 0" (Math|Vector|MakeVector _sizer _sizer _sizer))))))))

(fn SpawnBoxes
  (for _array_element (Variables|Default|GetPoints)
    (Class|InstancedStaticMeshComponent|AddInstanceWorldSpace (Variables|Default|GetHISMActor) _array_element)))