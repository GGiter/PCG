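; Player controller for a viewer that steps through fractal and landscape content with keys.
; N/P clear the current content and move through FractalArray; ActivateContentUI casts each entry, spawning a fractal or Julia actor with its widget, or showing only LandScapeUI.
; Other keys toggle the UI, open an exit screen or lock the camera.
; RotateCamera translates rather than rotates; the code assigning CameraActorRef and view target is disconnected from BeginPlay.
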(event EventBeginPlay
  (bind _outactors (Actor|GetAllActorsOfClass "/Script/Engine.CameraActor")))

(event Input|KeyboardEvents|P
  (params (Key :type Key%20Structure))
  (bind _contentref (Variables|Default|GetContentRef))
  (:Pressed
    (Utilities|IsValid _contentref
      (:Is%20Valid
        (Actor|DestroyActor _contentref))
      (:Is%20Not%20Valid
        _))
    (Viewport|RemoveAllWidgets)
    (if (and (< (+ -1 (Variables|Default|GetIndexFractalArray)) (Utilities|Array|Length (Variables|Default|GetFractalArray))) (> (+ -1 (Variables|Default|GetIndexFractalArray)) -1))
      (Variables|Default|SetIndexFractalArray (+ -1 (Variables|Default|GetIndexFractalArray)))
      (CallFunction|ActivateContentUI))))

(event Input|KeyboardEvents|A
  (params (Key :type Key%20Structure))
  (:Pressed
    (CallFunction|RotateCamera (Math|Vector|MakeVector 0.0 (* (Variables|Default|GetSpeed) -1.0) 0.0))))

(event Input|KeyboardEvents|S
  (params (Key :type Key%20Structure))
  (:Pressed
    (CallFunction|RotateCamera (Math|Vector|MakeVector (* (Variables|Default|GetSpeed) -1.0) 0.0 0.0))))

(event Input|KeyboardEvents|D
  (params (Key :type Key%20Structure))
  (:Pressed
    (CallFunction|RotateCamera (Math|Vector|MakeVector 0.0 (Variables|Default|GetSpeed) 0.0))))

(event Input|MouseEvents|MouseWheelUp
  (params (Key :type Key%20Structure))
  (:Pressed
    (CallFunction|RotateCamera (Math|Vector|MakeVector 0.0 0.0 (* (Variables|Default|GetSpeed) -1.0)))))

(event Input|KeyboardEvents|L
  (params (Key :type Key%20Structure))
  (:Pressed
    (Variables|Default|SetIsLocked (not (Variables|Default|GetIsLocked)))))

(event Input|KeyboardEvents|N
  (params (Key :type Key%20Structure))
  (bind _contentref (Variables|Default|GetContentRef))
  (:Pressed
    (Utilities|IsValid _contentref
      (:Is%20Valid
        (Actor|DestroyActor _contentref))
      (:Is%20Not%20Valid
        _))
    (Viewport|RemoveAllWidgets)
    (if (and (< (+ 1 (Variables|Default|GetIndexFractalArray)) (Utilities|Array|Length (Variables|Default|GetFractalArray))) (> (+ 1 (Variables|Default|GetIndexFractalArray)) -1))
      (Variables|Default|SetIndexFractalArray (+ 1 (Variables|Default|GetIndexFractalArray)))
      (CallFunction|ActivateContentUI))))

(event Input|KeyboardEvents|Q
  (params (Key :type Key%20Structure))
  (:Pressed
    (Viewport|RemoveAllWidgets)
    (bind _returnvalue (UserInterface|CreateWidget "/Game/Blueprints/UI/ExitUI.ExitUI_C"))
    (bind _output_get (Variables|Default|SetExitUIRef _returnvalue))
    (UserInterface|Viewport|AddtoViewport (Variables|Default|GetExitUIRef) 0)
    (Input|SetInputModeUIOnly self _output_get "DoNotLock")
    (Variables|Default|SetbShowMouseCursor true)))

(event Input|KeyboardEvents|W
  (params (Key :type Key%20Structure))
  (:Pressed
    (CallFunction|RotateCamera (Math|Vector|MakeVector (Variables|Default|GetSpeed) 0.0 0.0))))

(event Input|KeyboardEvents|U
  (params (Key :type Key%20Structure))
  (bind _contentuiref (Variables|Default|GetContentUIRef))
  (:Pressed
    (if (Widget|IsVisible _contentuiref)
      (Widget|SetVisibility _contentuiref "Hidden")
      (else
        (Widget|SetVisibility _contentuiref "Visible")))))

(event Input|MouseEvents|MouseWheelDown
  (params (Key :type Key%20Structure))
  (:Pressed
    (CallFunction|RotateCamera (Math|Vector|MakeVector 0.0 0.0 (Variables|Default|GetSpeed)))))

(fn ConstructionScript)

(fn RotateCamera
  (params (Vector :type Vector))
  (bind _cameraactorref (Variables|Default|GetCameraActorRef))
  (if (not (Variables|Default|GetIsLocked))
    (Transformation|SetActorLocation _cameraactorref (+ (Transformation|GetActorLocation _cameraactorref) Vector) false false)))

(fn ActivateContentUI
  (bind _fractalarray (Variables|Default|GetFractalArray))
  (bind _indexfractalarray (Variables|Default|GetIndexFractalArray))
  (bind _output (Utilities|Array|Get(acopy) _fractalarray _indexfractalarray))
  (bind _asfractal_actor (Utilities|Casting|CastToFractalActorClass _output)
    (:then
      (bind _returnvalue (UserInterface|CreateWidget "/Game/Blueprints/UI/BP_FractalUI.BP_FractalUI_C" self))
      (bind _returnvalue_2 (Game|SpawnActorfromClass _asfractal_actor (Math|Transform|MakeTransform "0, 0, 0") "Undefined" 0 0))
      (Variables|/Script/PCG.FractalUI|SetFractalRef _returnvalue _returnvalue_2)
      (Class|FractalUI|SetIsFractalSet _returnvalue true)
      (UserInterface|Viewport|AddtoViewport _returnvalue 0)
      (Variables|Default|SetContentUIRef _returnvalue)
      (Variables|Default|SetContentRef _returnvalue_2))
    (:CastFailed
      (bind _asbp_julia (Utilities|Casting|CastToBP_JuliaClass _output)
        (:then
          (bind _returnvalue_3 (Game|SpawnActorfromClass _asbp_julia (Math|Transform|MakeTransform "0, 0, 0") "Undefined" 0 0))
          (bind _returnvalue_4 (UserInterface|CreateWidget "/Game/Blueprints/UI/FractalTextUI.FractalTextUI_C" self))
          (Variables|/Game/Blueprints/UI/FractalTextUI.FractalTextUI_C|SetFractalRef _returnvalue_4 _returnvalue_3)
          (UserInterface|Viewport|AddtoViewport _returnvalue_4 0)
          (Variables|Default|SetContentUIRef _returnvalue_4)
          (Variables|Default|SetContentRef _returnvalue_3))
        (:CastFailed
          (bind _returnvalue_5 (UserInterface|CreateWidget "/Game/Blueprints/UI/LandScapeUI.LandScapeUI_C" self))
          (UserInterface|Viewport|AddtoViewport _returnvalue_5 0)
          (Variables|Default|SetContentUIRef _returnvalue_5))))))