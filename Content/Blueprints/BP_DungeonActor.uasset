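; BP_DungeonActor is a dungeon actor that runs Generate when play begins.
; A SetColors event loops over NumOfSections and applies NewMaterial to each section of its RuntimeMesh.
; The construction script computes box mesh data from a fixed-size GenerateBoxMesh call but never builds a mesh section from it here.
; Overlap and Tick events are disabled stubs.
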(event EventBeginPlay
  (PCG|Generate))

(event Collision|EventActorBeginOverlap
  (params (OtherActor :type Actor%20Object%20Reference)))

(event EventTick
  (params (DeltaSeconds :type Float%20%28single-precision%29)))

(event EventSetColors
  (for _index (range 0 (- (Variables|Default|GetNumOfSections) 1))
    (Rendering|Material|SetMaterial (Variables|Default|GetRuntimeMesh) _index "/Game/Blueprints/NewMaterial.NewMaterial")))

(fn ConstructionScript
  (bind (_vertices _triangles _normals _uvs _tangents) (Class|KismetProceduralMeshLibrary|GenerateBoxMesh "100.000000,100.000000,100.000000"))
  (Variables|Default|SetVertices _vertices)
  (Variables|Default|SetTriangles _triangles)
  (Variables|Default|SetNormals _normals)
  (Variables|Default|SetUVs _uvs)
  (Variables|Default|SetTangents _tangents))