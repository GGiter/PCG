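; BP_Julia is an item actor whose static mesh shows a parameterized material, apparently a Julia set judging by the name.
; The construction script applies the MaterialInst material, then pushes the stored offset and scale values into it as scalar parameters.
; UpdateOffset and UpdateScale set those parameters on the mesh's materials and store the new values, while the event graph holds no active logic.
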(event EventBeginPlay)

(event Collision|EventActorBeginOverlap
  (params (OtherActor :type Actor%20Object%20Reference)))

(event EventTick
  (params (DeltaSeconds :type Float%20%28single-precision%29)))

(fn ConstructionScript
  (Rendering|Material|SetMaterial (Variables|Default|GetStaticMesh) 0 (Variables|Default|GetMaterialInst))
  (CallFunction|UpdateOffset (Variables|Default|GetOffsetU) (Variables|Default|GetOffsetV))
  (CallFunction|UpdateScale (Variables|Default|GetScale)))

(fn UpdateOffset
  (params (OffsetU :type Float%20%28single-precision%29) (OffsetV :type Float%20%28single-precision%29))
  (bind _staticmesh (Variables|Default|GetStaticMesh))
  (Rendering|Material|SetScalarParameterValueonMaterials _staticmesh "OffsetU" OffsetU)
  (Rendering|Material|SetScalarParameterValueonMaterials _staticmesh "OffsetV" OffsetV)
  (Variables|Default|SetOffsetU OffsetU)
  (Variables|Default|SetOffsetV OffsetV))

(fn UpdateScale
  (params (Scale :type Float%20%28single-precision%29))
  (Rendering|Material|SetScalarParameterValueonMaterials (Variables|Default|GetStaticMesh) "Scale" Scale)
  (Variables|Default|SetScale Scale))