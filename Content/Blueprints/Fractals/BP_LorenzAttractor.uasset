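; Actor that visualizes a Lorenz attractor as a looping trail of small colored spheres flowing along its path.
; The construction script integrates the Lorenz equations with Euler steps via math expressions and feeds the points into a spline.
; BeginPlay creates one sphere per point with its own tinted material, then a restarting timeline moves them along the spline at staggered offsets.
; SpawnBeams can link spline points with beam emitters, but is not called here.
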(event Custom|MoveSphere
  (bind _spline (Variables|Default|GetSpline))
  (bind _animation (Timeline|Timeline_0 PlayFromStart)
    (:Update
      (for (_array_element _array_index) (Variables|Default|GetSpheres)
        (Transformation|SetWorldTransform _array_element (Math|Transform|MakeTransform (Spline|GetLocationatDistanceAlongSpline _spline (* (- _animation (* _array_index 0.001)) (Spline|GetSplineLength _spline)) "World") (Spline|GetRotationatDistanceAlongSpline _spline (* (- _animation (* _array_index 0.001)) (Spline|GetSplineLength _spline)) "World") "0.010000,0.010000,0.010000") false false)))
    (:Finished
      (CallFunction|MoveSphere))))

(event EventBeginPlay
  (for _index (range 0 (Utilities|Array|Length (Variables|Default|GetPoints)))
    (bind _returnvalue (AddComponent|AddStaticMeshComponent false))
    (bind _returnvalue_2 (Rendering|Material|CreateDynamicMaterialInstance _returnvalue 0 "/Game/LightMat_Inst.LightMat_Inst" :!class /Script/Engine.PrimitiveComponent))
    (Utilities|Array|Add (Variables|Default|GetSphereMat) _returnvalue_2)
    (Rendering|Material|SetVectorParameterValue _returnvalue_2 "Color" (Class|KismetMathLibrary|HSVtoRGB (Math|Conversions|ToFloat(Integer) _index) (+ (Math|Conversions|ToFloat(Integer) _index) (Math|Random|RandomFloatinRange 0.0 1e+01)) 1.0 1.0) :!class /Script/Engine.MaterialInstanceDynamic)
    (Transformation|SetWorldTransform _returnvalue (Math|Transform|MakeTransform "0, 0, 0" "0, 0, 0" "0.010000,0.010000,0.010000") false false)
    (Components|StaticMesh|SetStaticMesh _returnvalue "/Engine/EngineMeshes/MaterialSphere.MaterialSphere")
    (Utilities|Array|Add (Variables|Default|GetSpheres) _returnvalue))
  (CallFunction|MoveSphere))

(fn ConstructionScript
  (CallFunction|GeneratePoints)
  (for _array_element (Variables|Default|GetPoints)
    (Spline|AddSplinePoint (Variables|Default|GetSpline) _array_element "Local" false))
  (Spline|UpdateSpline (Variables|Default|GetSpline)))

(fn GeneratePoints
  (Utilities|Array|Clear (Variables|Default|GetPoints))
  (for _index (range 0 (Variables|Default|GetNumIterations))
    (bind _dx (CallFunction|DX (|((AA*(YY-XX))*DTT) (LocalVariables|GetA) (LocalVariables|GetX) (LocalVariables|GetY) (Variables|Default|GetDT)) (LocalVariables|GetX)))
    (bind _dy (CallFunction|DY (|(((XX*(BB-ZZ))-YY)*DTT) (LocalVariables|GetX) (LocalVariables|GetB) (LocalVariables|GetZ) (LocalVariables|GetY) (Variables|Default|GetDT)) (LocalVariables|GetY)))
    (bind _dz (CallFunction|DZ (|(((XX*YY)-(CC*ZZ))*DTT) (LocalVariables|GetX) (LocalVariables|GetY) (LocalVariables|GetC) (LocalVariables|GetZ) (Variables|Default|GetDT)) (LocalVariables|GetZ)))
    (LocalVariables|SetX _dx)
    (LocalVariables|SetY _dy)
    (LocalVariables|SetZ _dz)
    (Utilities|Array|Add (Variables|Default|GetPoints) (Math|Vector|MakeVector (LocalVariables|GetX) (LocalVariables|GetY) (LocalVariables|GetZ)))))

(fn DX
  (params (A :type Float%20%28single-precision%29) (B :type Float%20%28single-precision%29))
  (return (+ A B)))

(fn DY
  (params (A :type Float%20%28single-precision%29) (B :type Float%20%28single-precision%29))
  (return (+ A B)))

(fn DZ
  (params (A :type Float%20%28single-precision%29) (B :type Float%20%28single-precision%29))
  (return (+ A B)))

(fn SpawnBeams
  (bind _spline (Variables|Default|GetSpline))
  (for _index (range 0 (- (Spline|GetNumberOfSplinePoints _spline) 2))
    (bind _returnvalue (Effects|SpawnEmitteratLocation 0 "0, 0, 0"))
    (Effects|Components|ParticleSystem|SetVectorParameter _returnvalue "Source" (Spline|GetLocationatSplinePoint _spline _index "World"))
    (Effects|Components|ParticleSystem|SetVectorParameter _returnvalue "Source_Tan" (Spline|GetTangentatDistanceAlongSpline _spline (Spline|GetDistanceAlongSplineatSplinePoint _spline _index) "World"))
    (Effects|Components|ParticleSystem|SetVectorParameter _returnvalue "Target" (Spline|GetLocationatSplinePoint _spline (+ _index 1) "World"))
    (Effects|Components|ParticleSystem|SetVectorParameter _returnvalue "Target_Tan" (Spline|GetTangentatDistanceAlongSpline _spline (Spline|GetDistanceAlongSplineatSplinePoint _spline (+ _index 1)) "World"))))